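; bp_SpawnCharacter switches player control between characters already placed in the world; despite its name, it spawns nothing.
; Keys 1 and 2 find the first Bp_Character_Hook or Bp_DashCharacter, respectively, then player controller 0 unpossesses its current pawn and possesses that one.
; Any damage it receives destroys the first Bp_Minion found in the level, with no check that one exists.
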(event `self.ReceiveAnyDamage`
  (params (Damage :type "Float (single-precision)") (DamageType :type "DamageType Object Reference") (InstigatedBy :type "Controller Object Reference") (DamageCauser :type "Actor Object Reference"))
  (bind _outactors (`GameplayStatics.GetAllActorsOfClass` "/Game/Characters/bp_Minion.bp_Minion_C"))
  (`self.K2_DestroyActor` (`|GetArrayItem` _outactors)))

(event `self.ReceiveTick`
  (params (DeltaSeconds :type "Float (single-precision)")))

(event `Key|Two`
  (params (Key :type "Key Structure"))
  (bind _returnvalue (`GameplayStatics.GetPlayerController` 0))
  (:`Pressed`
    (bind _returnvalue_2 (`GameplayStatics.GetActorOfClass` "/Game/Characters/bp_DashCharacter.bp_DashCharacter_C"))
    (`Controller.UnPossess` _returnvalue)
    (`Controller.Possess` _returnvalue _returnvalue_2)))

(event `Key|One`
  (params (Key :type "Key Structure"))
  (bind _returnvalue (`GameplayStatics.GetPlayerController` 0))
  (:`Pressed`
    (bind _returnvalue_2 (`GameplayStatics.GetActorOfClass` "/Game/Characters/bp_Character_Hook.bp_Character_Hook_C"))
    (`Controller.UnPossess` _returnvalue)
    (`Controller.Possess` _returnvalue _returnvalue_2)))

(fn `UserConstructionScript`)